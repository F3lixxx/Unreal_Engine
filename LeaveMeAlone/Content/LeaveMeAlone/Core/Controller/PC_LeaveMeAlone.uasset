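; Player controller for LeaveMeAlone that handles pausing the game.
; It enables input on begin play and toggles on the IA_GamePause input action using an IsPauseMenuOpen flag.
; Opening creates a fresh WBP_Pause widget, adds it to the viewport and pauses the game; closing removes that widget and unpauses.
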(event Input|EnhancedActionEvents|EnhancedInputActionIA_GamePause
  (params (ActionValue :type Boolean) (ElapsedSeconds :type Float%20%28double-precision%29) (TriggeredSeconds :type Float%20%28double-precision%29) (InputAction :type Input%20Action%20Object%20Reference :default "/Game/LeaveMeAlone/Input/Input_Actions/IA_GamePause.IA_GamePause"))
  (:Started
    (if (not (Variables|Default|GetIsPauseMenuOpen))
      (Variables|Default|SetIsPauseMenuOpen true)
      (bind _returnvalue (UserInterface|CreateWidget "/Game/LeaveMeAlone/Widgets/UI/WBP_Pause.WBP_Pause_C" (Game|GetPlayerController 0)))
      (bind _output_get (Variables|Default|SetPauseMenuWidget _returnvalue))
      (UserInterface|Viewport|AddtoViewport _output_get 0)
      (Game|SetGamePaused true)
      (else
        ;[1 1 1] Exit Pause
        (Variables|Default|SetIsPauseMenuOpen false)
        (Widget|RemovefromParent (Variables|Default|GetPauseMenuWidget))
        (Game|SetGamePaused false)))))

(event EventBeginPlay
  (Input|EnableInput (Game|GetPlayerController 0)))

(fn ConstructionScript)